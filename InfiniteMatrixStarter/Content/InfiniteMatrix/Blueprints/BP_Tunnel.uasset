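; BP_Tunnel is a tunnel segment with a rotating holed wall that the player must pass through.
; RandomizeWall picks one of four hole meshes and a random roll, and Tick keeps the wall spinning.
; When the player overlaps the trigger zone, it spawns the next tunnel, destroys itself and adds score.
; Wall overlaps cost the player score and health, update the health bar and trigger restart on death, while projectiles are destroyed.
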(event OnComponentBeginOverlap(TriggerZone)
  (params (OverlappedComponent :type Primitive%20Component%20Object%20Reference) (OtherActor :type Actor%20Object%20Reference) (OtherComp :type Primitive%20Component%20Object%20Reference) (OtherBodyIndex :type Integer) (bFromSweep :type Boolean) (SweepResult :type Hit%20Result%20Structure%20%28by%20ref%29))
  ;[1 1 1] Passing Through the Hole
  (Utilities|FlowControl|Sequence
    (:then_0
      (Utilities|Casting|CastToBP_Player OtherActor)
      (Default|SpawnTunnelatSpawnPoint (Variables|Default|GetTunnelSpawner))
      (Actor|DestroyActor))
    (:then_1
      (bind _asbp_player (Utilities|Casting|CastToBP_Player OtherActor))
      ;;[1 1 1] Increase Player Score
      (bind _output_get (Variables|/Game/InfiniteMatrix/Blueprints/BP_Player.BP_Player_C|SetScore _asbp_player (+ (Variables|/Game/InfiniteMatrix/Blueprints/BP_Player.BP_Player_C|GetScore _asbp_player) 1)))
      (Default|UpdateScoreValue (Variables|/Game/InfiniteMatrix/Blueprints/BP_Player.BP_Player_C|GetScoreTextReference _asbp_player) _output_get))))

(event OnComponentBeginOverlap(WallMesh)
  (params (OverlappedComponent :type Primitive%20Component%20Object%20Reference) (OtherActor :type Actor%20Object%20Reference) (OtherComp :type Primitive%20Component%20Object%20Reference) (OtherBodyIndex :type Integer) (bFromSweep :type Boolean) (SweepResult :type Hit%20Result%20Structure%20%28by%20ref%29))
  ;[1 1 1] Wall Collision Handling
  (Utilities|FlowControl|Sequence
    (:then_0
      ;;[1 1 1] Decrement Score
      (bind _asbp_player (Utilities|Casting|CastToBP_Player OtherActor))
      (Variables|/Game/InfiniteMatrix/Blueprints/BP_Player.BP_Player_C|SetScore _asbp_player (- (Variables|/Game/InfiniteMatrix/Blueprints/BP_Player.BP_Player_C|GetScore _asbp_player) 1)))
    (:then_1
      (bind _asbp_player_2 (Utilities|Casting|CastToBP_Player OtherActor))
      ;;[1 1 1] Decrease Player Health
      (bind _output_get (Variables|/Game/InfiniteMatrix/Blueprints/BP_Player.BP_Player_C|SetCurrentHealth _asbp_player_2 (- (Variables|/Game/InfiniteMatrix/Blueprints/BP_Player.BP_Player_C|GetCurrentHealth _asbp_player_2) 1e+01)))
      ;;[1 1 1] HUD Updates
      (Default|UpdateHealthBar (Variables|/Game/InfiniteMatrix/Blueprints/BP_Player.BP_Player_C|GetHealthBarReference _asbp_player_2) _output_get (Variables|/Game/InfiniteMatrix/Blueprints/BP_Player.BP_Player_C|GetMaxHealth _asbp_player_2))
      (Default|UpdateColor (Variables|/Game/InfiniteMatrix/Blueprints/BP_Player.BP_Player_C|GetHealthBarReference _asbp_player_2) _output_get (Variables|/Game/InfiniteMatrix/Blueprints/BP_Player.BP_Player_C|GetMaxHealth _asbp_player_2))
      (if (<= _output_get 0.0)
        (Variables|/Game/InfiniteMatrix/Blueprints/BP_Player.BP_Player_C|SetIsDead _asbp_player_2 true)
        (Default|DisplayRestart _asbp_player_2)))
    (:then_2
      ;;[1 1 1] Cleanup Projectile
      (bind _asbp_projectile (Utilities|Casting|CastToBP_Projectile OtherActor))
      (Default|DestroyProjectile _asbp_projectile))))

(event EventTick
  (params (DeltaSeconds :type Float%20%28single-precision%29))
  ;[1 1 1] Rotate Wall to add Difficulty
  (Transformation|AddLocalRotation (Variables|Default|GetWallMesh) (Math|Rotator|MakeRotator (* DeltaSeconds (Variables|Default|GetRotateSpeed)) 0.0 0.0) false false))

(fn ConstructionScript)

(fn RandomizeWall
  ;[1 1 1] Randomly Choose a Wall Pattern
  (Components|StaticMesh|SetStaticMesh (Variables|Default|GetWallMesh) (Utilities|Select :Index (Math|Random|RandomIntegerinRange 0 3) :Option%200 "/Game/InfiniteMatrix/Meshes/SM_Hole_01.SM_Hole_01" :Option%201 "/Game/InfiniteMatrix/Meshes/SM_Hole_02.SM_Hole_02" :Option%202 "/Game/InfiniteMatrix/Meshes/SM_Hole_03.SM_Hole_03" :Option%203 "/Game/InfiniteMatrix/Meshes/SM_Hole_04.SM_Hole_04"))
  (Transformation|AddLocalRotation (Variables|Default|GetWallMesh) (Math|Rotator|MakeRotator (Math|Random|RandomFloatinRange 0.0 3.6e+02) 0.0 0.0) false false))