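; BP_Projectile is an accelerating projectile actor that is destroyed when it hits tunnel or health pack actors.
; Each Tick adds a fixed increment to ForwardSpeed and offsets the actor along world X, so acceleration depends on frame rate.
; The Cylinder's begin-overlap event casts for BP_Tunnel and BP_HealthPack to destroy the projectile.
; A separate DestroyProjectile function also destroys the actor, though nothing in this Blueprint calls it.
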(event OnComponentBeginOverlap(Cylinder)
  (params (OverlappedComponent :type Primitive%20Component%20Object%20Reference) (OtherActor :type Actor%20Object%20Reference) (OtherComp :type Primitive%20Component%20Object%20Reference) (OtherBodyIndex :type Integer) (bFromSweep :type Boolean) (SweepResult :type Hit%20Result%20Structure%20%28by%20ref%29))
  ;[1 1 1] Collision with Non-Enemy
  (Utilities|FlowControl|Sequence
    (:then_0
      (Utilities|Casting|CastToBP_Tunnel OtherActor)
      (Actor|DestroyActor self))
    (:then_1
      (Utilities|Casting|CastToBP_HealthPack OtherActor)
      (Actor|DestroyActor self))))

(event EventTick
  (params (DeltaSeconds :type Float%20%28single-precision%29))
  ;[1 1 1] Make Projectile Move
  (bind _output_get (Variables|Default|SetForwardSpeed (+ (Variables|Default|GetForwardSpeed) 1e+01)))
  (Transformation|AddActorWorldOffset (Math|Vector|MakeVector (* _output_get DeltaSeconds) 0.0 0.0)))

(fn ConstructionScript)

(fn DestroyProjectile
  (Actor|DestroyActor))